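; Trigger volume that makes the player's flashlight flicker when they walk in with it switched on, optionally only once.
; On overlap it plays an attached sound and drives the spotlight intensity through a timeline, guarded by a CanDoFlicker flag.
; A work-in-progress WithAnimation branch also plays a first-person montage after a short delay.
; The construction script scales the trigger box from its length, thickness and height variables.
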(event `self.ReceiveBeginPlay`
  ;[0.05098 0.05098 0.05098] Cast to Player
  (bind _asbp_fpmovement_player (cast `/Game/FPMovement/Player/Blueprints/BP_FPMovementPlayer` (`GameplayStatics.GetPlayerCharacter` 0)))
  (set `self.Player Reference` _asbp_fpmovement_player))

(event `self.TriggerBox.OnComponentBeginOverlap`
  (params (OverlappedComponent :type "PrimitiveComponent Object Reference") (OtherActor :type "Actor Object Reference") (OtherComp :type "PrimitiveComponent Object Reference") (OtherBodyIndex :type Integer) (bFromSweep :type Boolean) (SweepResult :type "HitResult Structure (by ref)"))
  ;[0.05098 0.05098 0.05098] Flashlight Flicker function
  (bind _asbp_fpmovement_player (cast `/Game/FPMovement/Player/Blueprints/BP_FPMovementPlayer` OtherActor))
  (if (`/Game/FPMovement/Player/Blueprints/BP_FPMovementPlayer.FlashlightOn?` _asbp_fpmovement_player)
    (if (`self.Do Once?`)
      (`/Engine/EditorBlueprintResources/StandardMacros.DoOnce` false
        (:`Completed`
          (if (`self.Can Do Flicker`)
            (set `self.Can Do Flicker` false)
            (if (`self.With Animation? `)
              ;;[0.05098 0.05098 0.05098] with Animation [WIP]
              (`GameplayStatics.SpawnSoundAttached` (`self.Flicker SFX`) (`/Game/FPMovement/Player/Blueprints/BP_FPMovementPlayer.Flashlight` (`self.Player Reference`)) "None" (0.0 0.0 0.0) (struct) "KeepRelativeOffset" false (`self.Flicker SFX Volume`) 1.0 0.0 "/Game/FPMovement/Audio/Abilitys/Pickup/Effects/ItemAttenuation.ItemAttenuation" null)
              (bind (_direction _alpha) (`Timeline|Timeline` :!via `PlayFromStart`)
                (:`Update`
                  (`LightComponent.SetIntensity` (`/Game/FPMovement/Player/Blueprints/BP_FPMovementPlayer.SpotLight` (`self.Player Reference`)) (`KismetMathLibrary.Lerp` 0.0 (`/Game/FPMovement/Player/Blueprints/BP_FPMovementPlayer.FlashlightIntensity` (`self.Player Reference`)) _alpha))
                  (`KismetSystemLibrary.Delay` 0.45)
                  (`|PlayMontage` (`/Game/FPMovement/Player/Blueprints/BP_FPMovementPlayer.FirstPersonMesh` (`self.Player Reference`)) (`self.Animation`)
                    (:`OnBlendOut`
                      (set `self.Can Do Flicker` true)))))
              (else
                ;;[0.05098 0.05098 0.05098] without Animation
                (`GameplayStatics.SpawnSoundAttached` (`self.Flicker SFX`) (`/Game/FPMovement/Player/Blueprints/BP_FPMovementPlayer.Flashlight` (`self.Player Reference`)) "None" (0.0 0.0 0.0) (struct) "KeepRelativeOffset" false (`self.Flicker SFX Volume`) 1.0 0.0 "/Game/FPMovement/Audio/Abilitys/Pickup/Effects/ItemAttenuation.ItemAttenuation" null)
                (bind (_direction_2 _alpha_2) (`Timeline|Flicker_TL` :!via `PlayFromStart`)
                  (:`Update`
                    (`LightComponent.SetIntensity` (`/Game/FPMovement/Player/Blueprints/BP_FPMovementPlayer.SpotLight` (`self.Player Reference`)) (`KismetMathLibrary.Lerp` 0.0 (`/Game/FPMovement/Player/Blueprints/BP_FPMovementPlayer.FlashlightIntensity` (`self.Player Reference`)) _alpha_2))
                    (set `self.Can Do Flicker` true))))))))
      (elif (`self.Can Do Flicker`)
        (set `self.Can Do Flicker` false)
        (if (`self.With Animation? `)
          ;;[0.05098 0.05098 0.05098] with Animation [WIP]
          (`GameplayStatics.SpawnSoundAttached` (`self.Flicker SFX`) (`/Game/FPMovement/Player/Blueprints/BP_FPMovementPlayer.Flashlight` (`self.Player Reference`)) "None" (0.0 0.0 0.0) (struct) "KeepRelativeOffset" false (`self.Flicker SFX Volume`) 1.0 0.0 "/Game/FPMovement/Audio/Abilitys/Pickup/Effects/ItemAttenuation.ItemAttenuation" null)
          (bind (_direction_3 _alpha_3) (`Timeline|Timeline_1` :!via `PlayFromStart`)
            (:`Update`
              (`LightComponent.SetIntensity` (`/Game/FPMovement/Player/Blueprints/BP_FPMovementPlayer.SpotLight` (`self.Player Reference`)) (`KismetMathLibrary.Lerp` 0.0 (`/Game/FPMovement/Player/Blueprints/BP_FPMovementPlayer.FlashlightIntensity` (`self.Player Reference`)) _alpha_3))
              (`KismetSystemLibrary.Delay` 0.45)
              (`|PlayMontage` (`/Game/FPMovement/Player/Blueprints/BP_FPMovementPlayer.FirstPersonMesh` (`self.Player Reference`)) (`self.Animation`)
                (:`OnBlendOut`
                  (set `self.Can Do Flicker` true)))))
          (else
            ;;[0.05098 0.05098 0.05098] without Animation
            (`GameplayStatics.SpawnSoundAttached` (`self.Flicker SFX`) (`/Game/FPMovement/Player/Blueprints/BP_FPMovementPlayer.Flashlight` (`self.Player Reference`)) "None" (0.0 0.0 0.0) (struct) "KeepRelativeOffset" false (`self.Flicker SFX Volume`) 1.0 0.0 "/Game/FPMovement/Audio/Abilitys/Pickup/Effects/ItemAttenuation.ItemAttenuation" null)
            (bind (_direction_4 _alpha_4) (`Timeline|Timeline_0` :!via `PlayFromStart`)
              (:`Update`
                (`LightComponent.SetIntensity` (`/Game/FPMovement/Player/Blueprints/BP_FPMovementPlayer.SpotLight` (`self.Player Reference`)) (`KismetMathLibrary.Lerp` 0.0 (`/Game/FPMovement/Player/Blueprints/BP_FPMovementPlayer.FlashlightIntensity` (`self.Player Reference`)) _alpha_4))
                (set `self.Can Do Flicker` true)))))))
    (else
      (`KismetSystemLibrary.PrintText` "Flashlight not in use"))))

(fn `UserConstructionScript`
  (`SceneComponent.SetWorldScale3D` (`self.TriggerBox`) (`KismetMathLibrary.MakeVector` (`self.Box Length`) (`self.Box Thickness`) (`self.Box Height`))))