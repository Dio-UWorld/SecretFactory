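; BP_BaseKey is a base key pickup for the door system of the first-person movement player.
; On BeginPlay it caches the player character as a BP_FPMovementPlayer reference.
; Interact adds its KeyID to the player's DoorKeys, plays a pickup sound at the item's location with attenuation, then destroys the actor.
; The construction script applies a configurable mesh and scale to the Item component.
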(event `self.ReceiveBeginPlay`
  ;[0.05098 0.05098 0.05098] Cast to Player
  (bind _asbp_fpmovement_player (cast `/Game/FPMovement/Player/Blueprints/BP_FPMovementPlayer` (`GameplayStatics.GetPlayerCharacter` 0)))
  (set `self.Player Reference` _asbp_fpmovement_player))

(event `Play Pickup SFX`
  ;[0.05098 0.05098 0.05098] Custom Events
  (`GameplayStatics.PlaySoundAtLocation` (`self.Pickup SFX`) (`SceneComponent.K2_GetComponentLocation` (`self.Item`)) (struct) (`self.Pickup Volume`) 1.0 0.0 "/Game/FPMovement/Audio/Abilitys/Pickup/Effects/ItemAttenuation.ItemAttenuation" null null null))

(event `self.BP_Interact`
  (params (FPMovementPlayer :type "/Game/FPMovement/Player/Blueprints/BP_FPMovementPlayer Object Reference"))
  ;[0.05098 0.05098 0.05098] Key function
  (`KismetArrayLibrary.Array_Add` (`/Game/FPMovement/Player/Blueprints/BP_FPMovementPlayer.DoorKeys` (`self.Player Reference`)) (`self.KeyID`))
  (`self.Play Pickup SFX`)
  (`self.K2_DestroyActor`))

(fn `UserConstructionScript`
  (`StaticMeshComponent.SetStaticMesh` (`self.Item`) (`self.Key Mesh`))
  (`SceneComponent.SetWorldScale3D` (`self.Item`) (`KismetMathLibrary.Conv_DoubleToVector` (`self.Key Scale`))))