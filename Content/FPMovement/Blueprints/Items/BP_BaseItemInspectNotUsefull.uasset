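; BP_BaseItemInspectNotUsefull is an inspectable item for the first-person player, with configurable mesh, scale and pickup sound.
; A one-time Interact plays the sound, shows the cursor, locks movement and look, and a timeline lerps the item to the player's ItemInspect transform.
; While inspection is enabled, Tick and MouseX share a branch that rotates the item from mouse axis values.
; The graph has no logic to end inspection or restore control.
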(event `Play Pickup SFX`
  ;[0.05098 0.05098 0.05098] Custom Events
  (`GameplayStatics.PlaySoundAtLocation` (`self.Pickup SFX`) (`SceneComponent.K2_GetComponentLocation` (`self.Item`)) (struct) (`self.Pickup Volume`) 1.0 0.0 "/Game/FPMovement/Audio/Abilitys/Pickup/Effects/ItemAttenuation.ItemAttenuation" null null null))

(event `self.ReceiveTick`
  (params (DeltaSeconds :type "Float (single-precision)"))
  (if (`self.Can Inspect?`) :!label _label
    (`SceneComponent.K2_AddLocalRotation` (`self.Item`) (`KismetMathLibrary.MakeRotator` (* (stale `InputAxisKey|MouseX` AxisValue) 0.4) (* (stale `InputAxisKey|MouseY` AxisValue) -0.4)) false false)))

(event `InputAxisKey|MouseX`
  (params (AxisValue :type "Float (single-precision)"))
  (goto _label))

(event `InputAxisKey|MouseY`
  (params (AxisValue :type "Float (single-precision)")))

(event `self.ReceiveBeginPlay`
  (bind _item (`self.Item`))
  ;[0.05098 0.05098 0.05098] Cast to Player
  (bind _output_get (set `self.Original Location` (`SceneComponent.K2_GetComponentLocation` _item)))
  (bind _output_get_2 (set `self.Original Rotation` (`SceneComponent.K2_GetComponentRotation` _item)))
  (`self.EnableInput` (`GameplayStatics.GetPlayerController` 0)))

(event `self.BP_Interact`
  (params (FPMovementPlayer :type "/Game/FPMovement/Player/Blueprints/BP_FPMovementPlayer Object Reference"))
  (`/Engine/EditorBlueprintResources/StandardMacros.DoOnce` false
    (:`Completed`
      (set `PlayerController.bShowMouseCursor` true (`GameplayStatics.GetPlayerController` 0))
      (set `self.Can Inspect?` true)
      ;[0.05098 0.05098 0.05098] Pickup/Destroy function
      (bind _asbp_fpmovement_player (cast `/Game/FPMovement/Player/Blueprints/BP_FPMovementPlayer` (`GameplayStatics.GetPlayerCharacter` 0)))
      (if true
        (`self.Play Pickup SFX`)
        (`CharacterMovementComponent.DisableMovement` (`Character.CharacterMovement` (`GameplayStatics.GetPlayerCharacter` 0)))
        (`Controller.SetIgnoreLookInput` (`GameplayStatics.GetPlayerController` 0) true)
        (bind (_direction _newtrack_0) (`Timeline|Timeline` :!via `PlayFromStart`)
          (:`Update`
            (bind (_returnvalue_location _returnvalue_rotation) (`KismetMathLibrary.BreakTransform` (`SceneComponent.K2_GetComponentToWorld` (`/Game/FPMovement/Player/Blueprints/BP_FPMovementPlayer.ItemInspect` _asbp_fpmovement_player))))
            (`SceneComponent.K2_SetWorldTransform` (`self.Item`) (`KismetMathLibrary.MakeTransform` (`KismetMathLibrary.VLerp` (stale `self.ReceiveBeginPlay` _output_get) _returnvalue_location _newtrack_0) (`KismetMathLibrary.RLerp` (stale `self.ReceiveBeginPlay` _output_get_2) _returnvalue_rotation _newtrack_0)) false false)))))))

(fn `UserConstructionScript`
  (`StaticMeshComponent.SetStaticMesh` (`self.Item`) (`self.Item Mesh`))
  (`SceneComponent.SetWorldScale3D` (`self.Item`) (`KismetMathLibrary.Conv_DoubleToVector` (`self.Item Scale`))))