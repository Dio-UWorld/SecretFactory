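; Base inspectable item for the FPMovement player, intended as a parent for specific items that add their own interaction logic.
; The construction script applies the configured mesh and scale, and BeginPlay caches the player reference.
; When Inspect is set, Interact plays an attenuated pickup sound and spawns a BP_InspectItem far off-world.
; It passes that actor the mesh, name, description, inspection rotation and scale.
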(event `self.ReceiveBeginPlay`
  ;[0.05098 0.05098 0.05098] Cast to Player
  (bind _asbp_fpmovement_player (cast `/Game/FPMovement/Player/Blueprints/BP_FPMovementPlayer` (`GameplayStatics.GetPlayerCharacter` 0)))
  (set `self.Player Reference` _asbp_fpmovement_player))

(event `Play Pickup SFX`
  ;[0.05098 0.05098 0.05098] Custom Events
  (`GameplayStatics.PlaySoundAtLocation` (`self.Pickup SFX`) (`SceneComponent.K2_GetComponentLocation` (`self.Item`)) (struct) (`self.Pickup Volume`) 1.0 0.0 "/Game/FPMovement/Audio/Abilitys/Pickup/Effects/ItemAttenuation.ItemAttenuation" null null null))

(event `self.BP_Interact`
  (params (FPMovementPlayer :type "/Game/FPMovement/Player/Blueprints/BP_FPMovementPlayer Object Reference"))
  ;[0.05098 0.05098 0.05098] Pickup/Destroy function
  (if (`self.Inspect?`)
    (`self.Play Pickup SFX`)
    (bind _returnvalue (`|SpawnActorFromClass` "/Game/FPMovement/Blueprints/Items/BP_InspectItem.BP_InspectItem_C" (`KismetMathLibrary.MakeTransform` (1e+17 0.0 0.0)) "Undefined" "MultiplyWithRoot" null null))
    (`/Game/FPMovement/Blueprints/Items/BP_InspectItem.SET Inspect Rotation` _returnvalue (`self.Item Inspection Rotaion`))
    (`/Game/FPMovement/Blueprints/Items/BP_InspectItem.Set Inspect Scale` _returnvalue (`self.Item Inspection Scale`))
    (message `/Game/FPMovement/Player/Blueprints/Interface/BP_Interact.Inspect` _returnvalue FPMovementPlayer (`StaticMeshComponent.StaticMesh` (`self.Item`)) (`self.Item Name`) (`self.Item Descriptiton`))))

(fn `UserConstructionScript`
  (bind _item (`self.Item`))
  (`|ExecutionSequence`
    (:`then_0`
      (`StaticMeshComponent.SetStaticMesh` (`self.Item`) (`self.Item Mesh`))
      (`SceneComponent.K2_SetWorldTransform` _item (`KismetMathLibrary.MakeTransform` (`SceneComponent.K2_GetComponentLocation` _item) (`SceneComponent.K2_GetComponentRotation` _item) (`self.Item Scale`)) false false))))