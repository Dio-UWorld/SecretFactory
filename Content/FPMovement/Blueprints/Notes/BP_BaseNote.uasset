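; Base actor for readable notes in the FPMovement game, with a configurable mesh and scale applied in the construction script.
; On interact it opens a note widget fed by its data asset, plays a positional read sound and switches to UI-only input with the cursor shown.
; Flags optionally add the data asset to the player's note array without duplicates, or destroy the actor after reading.
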(event `self.ReceiveBeginPlay`
  ;[0.05098 0.05098 0.05098] Cast to Player
  (bind _asbp_fpmovement_player (cast `/Game/FPMovement/Player/Blueprints/BP_FPMovementPlayer` (`GameplayStatics.GetPlayerCharacter` 0)))
  (set `self.Player Reference` _asbp_fpmovement_player))

(event `Play Note SFX`
  ;[0.05098 0.05098 0.05098] Custom Events
  (`GameplayStatics.PlaySoundAtLocation` (`self.Read Note SFX`) (`SceneComponent.K2_GetComponentLocation` (`self.Note`)) (struct) (`self.Read Note Volume`) 1.0 0.0 "/Game/FPMovement/Audio/Abilitys/Pickup/Effects/ItemAttenuation.ItemAttenuation" null null null))

(event `self.BP_Interact`
  (params (FPMovementPlayer :type "/Game/FPMovement/Player/Blueprints/BP_FPMovementPlayer Object Reference"))
  ;[0.05098 0.05098 0.05098] Interact w/ Note function
  (bind _dataasset (`self.DataAsset`)
    (:`then`
      (bind _returnvalue (`|CreateWidget` "/Game/FPMovement/Player/Widgets/UserCreated/WB_Note.WB_Note_C" null _dataasset))
      (bind _output_get (set `self.WB Note` _returnvalue))
      (`UserWidget.AddToViewport` _output_get 0)
      (`self.Play Note SFX`)
      (`WidgetBlueprintLibrary.SetInputMode_UIOnlyEx` (`GameplayStatics.GetPlayerController` 0) null)
      (set `PlayerController.bShowMouseCursor` true (`GameplayStatics.GetPlayerController` 0))
      (if (`self.SaveNote?`)
        (`KismetArrayLibrary.Array_AddUnique` (`/Game/FPMovement/Player/Blueprints/BP_FPMovementPlayer.NoteArray` FPMovementPlayer) (`self.DataAsset`)))
      (if (`self.DestroyOnRead?`)
        (`/Engine/EditorBlueprintResources/StandardMacros.IsValid` self
          (:`Is Valid`
            (`self.K2_DestroyActor`)))))
    (:`else`)))

(fn `UserConstructionScript`
  (`StaticMeshComponent.SetStaticMesh` (`self.Note`) (`self.Note Mesh`))
  (`SceneComponent.SetWorldScale3D` (`self.Note`) (`KismetMathLibrary.Conv_DoubleToVector` (`self.Note Scale`))))